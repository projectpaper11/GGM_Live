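; BP_F1GameMode is the game mode for a target-shooting game, handling target spawning, play time and the end-of-game result.
; A self-rescheduling timer spawns red (about 20% chance) or blue targets at random TriggerBox transforms, with delay read from a curve over play time.
; GameResult pauses the game, saves any new high score to the save slot loaded at BeginPlay, and shows a widget with score, time and accuracy.
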(event `self.ReceiveBeginPlay`
  (`|ExecutionSequence`
    (:`then_0`
      (bind _outactors (`GameplayStatics.GetAllActorsOfClass` "/Script/Engine.TriggerBox"))
      (set `self.TriggerBoxes` _outactors)
      (`KismetSystemLibrary.K2_SetTimerDelegate` (`|CreateDelegate` :!event `RandomSpawnTarget`) (`CurveFloat.GetFloatValue` (`self.SpawnDelayCurve`) (`self.PlayTime`))))
    (:`then_1`
      (bind _returnvalue (`GameplayStatics.DoesSaveGameExist` "GameResult"))
      (if _returnvalue
        (bind _returnvalue_2 (`GameplayStatics.LoadGameFromSlot` "GameResult"))
        (bind _assg_result (cast `/Game/GameData/SaveGame/SG_Result` _returnvalue_2))
        (set `self.HighScore` (`/Game/GameData/SaveGame/SG_Result.HighScore` _assg_result))))))

(event `self.ReceiveTick`
  (params (DeltaSeconds :type "Float (single-precision)"))
  (set `self.PlayTime` (+ DeltaSeconds (`self.PlayTime`))))

(fn `GameResult`
  (`GameplayStatics.SetGamePaused` true)
  (`|ExecutionSequence`
    (:`then_0`
      (bind _returnvalue (`|CreateWidget` "/Game/UI/WBP_GameResult.WBP_GameResult_C"))
      (bind _output_get (set `self.GameResultWidget` _returnvalue))
      (`UserWidget.AddToViewport` _output_get 0)
      (`WidgetBlueprintLibrary.SetInputMode_UIOnlyEx` (`GameplayStatics.GetPlayerController` 0) null)
      (set `PlayerController.bShowMouseCursor` true (`GameplayStatics.GetPlayerController` 0)))
    (:`then_1`
      (if (> (`self.Score`) (`self.HighScore`))
        (set `self.HighScore` (`self.Score`))
        (bind _returnvalue_2 (`GameplayStatics.CreateSaveGameObject` "/Game/GameData/SaveGame/SG_Result.SG_Result_C"))
        (set `self.SaveGameResult` _returnvalue_2)
        (set `/Game/GameData/SaveGame/SG_Result.HighScore` (`self.HighScore`) (`self.SaveGameResult`))
        (`GameplayStatics.SaveGameToSlot` (`self.SaveGameResult`) "GameResult")))
    (:`then_2`
      (`/Game/UI/WBP_GameResult.Update` (`self.GameResultWidget`) (`self.Score`) (`KismetMathLibrary.FTrunc` (`self.PlayTime`)) (`self.HighScore`) (`KismetMathLibrary.FTrunc` (* (/ (`KismetMathLibrary.Conv_IntToDouble` (`self.HitCount`)) (`KismetMathLibrary.Conv_IntToDouble` (`self.FireCount`))) 100.0))))))

(fn `RandomSpawnTarget`
  (`|ExecutionSequence`
    (:`then_0`
      (if (<= (`KismetMathLibrary.RandomFloatInRange` 0.0 100.0) 20.0)
        (set `self.SpawnActorClass` "/Game/Blueprints/Target/BP_F1TargetRed.BP_F1TargetRed_C")
        (else
          (set `self.SpawnActorClass` "/Game/Blueprints/Target/BP_F1TargetBlue.BP_F1TargetBlue_C"))))
    (:`then_1`
      (`|SpawnActorFromClass` (`self.SpawnActorClass`) (`self.GetTransform` (`|GetArrayItem` (`self.TriggerBoxes`) (`KismetMathLibrary.RandomIntegerInRange` 0 (- (`KismetArrayLibrary.Array_Length` (`self.TriggerBoxes`)) 1)))) "Undefined" "MultiplyWithRoot" null null)
      (bind _returnvalue (`KismetSystemLibrary.K2_SetTimerDelegate` (`|CreateDelegate` :!event `RandomSpawnTarget`) (`CurveFloat.GetFloatValue` (`self.SpawnDelayCurve`) (`self.PlayTime`))))
      (set `self.SpawnTimerHandle` _returnvalue))))

(fn `UserConstructionScript`)